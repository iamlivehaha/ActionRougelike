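; LeverBP is an interactable lever actor that triggers other actors in the level.
; On Interact, a FlipFlop pitches the handle mesh back and forth, then forwards the Interact interface message to SelectedActor with the instigating pawn.
; It also directly casts TrapActor to RedBarrel_BP to call Explode, gated on IsActorBeingDestroyed returning true, a path marked as unsafe.
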(event EventBeginPlay)

(event Collision|EventActorBeginOverlap
  (params (OtherActor :type Actor%20Object%20Reference)))

(event EventTick
  (params (DeltaSeconds :type Float%20%28single-precision%29)))

(event EventInteract
  (params (InstigatorPawn :type Pawn%20Object%20Reference))
  (bind _handlemesh (Variables|Default|GetHandleMesh))
  (bind _trapactor (Variables|Default|GetTrapActor))
  (Utilities|FlowControl|FlipFlop
    (:A
      (Transformation|AddRelativeRotation _handlemesh (Math|Rotator|MakeRotator 0.0 -5e+01 0.0) false false))
    (:B
      (Transformation|AddRelativeRotation _handlemesh (Math|Rotator|MakeRotator 0.0 5e+01 0.0) false false)))
  (Class|SGamePlayInterface|Interact(Message) (Variables|Default|GetSelectedActor) InstigatorPawn)
  (if (Game|IsActorBeingDestroyed _trapactor)
    (bind _asred_barrel_bp (Utilities|Casting|CastToRedBarrel_BP _trapactor))
    (Default|Explode _asred_barrel_bp)))

(fn ConstructionScript)