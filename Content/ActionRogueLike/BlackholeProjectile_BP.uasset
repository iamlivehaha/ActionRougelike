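; Black hole projectile that destroys physics-simulating actors it touches.
; On BeginPlay its sphere component ignores the first player's pawn while moving, and a timer destroys the projectile after a few seconds.
; When the sphere begins overlapping an actor, that actor is destroyed if its root component simulates physics.
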(event OnComponentBeginOverlap(SphereComp)
  (params (OverlappedComponent :type Primitive%20Component%20Object%20Reference) (OtherActor :type Actor%20Object%20Reference) (OtherComp :type Primitive%20Component%20Object%20Reference) (OtherBodyIndex :type Integer) (bFromSweep :type Boolean) (SweepResult :type Hit%20Result%20Structure%20%28by%20ref%29))
  (if (Physics|IsSimulatingPhysics (Variables|/Script/Engine.Actor|GetRootComponent OtherActor) "None")
    (Actor|DestroyActor OtherActor)))

(event Custom|Destory
  (Actor|DestroyActor))

(event EventBeginPlay
  (Collision|IgnoreActorwhenMoving (Variables|Default|GetSphereComp) (Game|Player|GetPlayerPawn 0) true)
  (Utilities|Time|SetTimerbyEvent (delegate Custom|Destory) 5.0))

(fn ConstructionScript)